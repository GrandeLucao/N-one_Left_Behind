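; Enemy character that roams the level, then chases and shoots the player character when it sees it.
; From BeginPlay it moves to random reachable nearby points, picking another after each successful move.
; PawnSensing sightings of a ThirdPersonCharacter turn it toward the target, issue an AI move to it and spawn a Bullet at the Scene component.
; A ShootDelay flag with a Delay throttles the fire rate.
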(event OnSeePawn(PawnSensing)
  (params (Pawn :type Pawn%20Object%20Reference))
  (bind _asthird_person_character (Utilities|Casting|CastToThirdPersonCharacter Pawn))
  (Utilities|FlowControl|Sequence
    (:then_0
      (Transformation|SetActorRotation (Math|Rotator|FindLookatRotation (Transformation|GetActorLocation) (Transformation|GetActorLocation _asthird_person_character)))
      (AI|AIMoveTo self "0, 0, 0" _asthird_person_character 5.0 false))
    (:then_1
      (if (Variables|Default|GetshootDelay)
        (Game|SpawnActorfromClass "/Game/Enemy/Bullet.Bullet_C" (Transformation|GetWorldTransform (Variables|Default|GetScene)) "Undefined" 0 0)
        (Variables|Default|SetshootDelay false)
        (Utilities|FlowControl|Delay 1.0)
        (Variables|Default|SetshootDelay true)))))

(event Custom|RandomRoam
  (AI|AIMoveTo self (.RandomLocation (AI|Navigation|GetRandomReachablePointinRadius (Transformation|GetActorLocation) 2e+03 0 0)) 0 5.0 false
    (:OnSuccess
      (CallFunction|RandomRoam))))

(event EventBeginPlay
  (CallFunction|RandomRoam))

(event Collision|EventActorBeginOverlap
  (params (OtherActor :type Actor%20Object%20Reference)))

(event EventTick
  (params (DeltaSeconds :type Float%20%28single-precision%29)))

(fn ConstructionScript)